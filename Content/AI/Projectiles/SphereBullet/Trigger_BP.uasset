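; Chaos field actor for the SphereBullet projectile that breaks and scatters destructible geometry.
; Explode applies an external cluster strain field through a radial falloff sized and centered on its Sphere component.
; It then applies a radial linear velocity field, culled outside that same sphere, to push pieces outward.
; The actor destroys itself immediately afterward.
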(event Custom|Explode
  (bind _fieldsystemcomponent (Variables|Field|GetFieldSystemComponent))
  (bind _radialfalloff (Variables|Default|GetRadialFalloff))
  (bind _sphere (Variables|Default|GetSphere))
  (bind _returnvalue (Components|Sphere|GetScaledSphereRadius _sphere))
  (bind _returnvalue_2 (Transformation|GetWorldLocation _sphere))
  (bind _returnvalue_3 (Field|SetRadialFalloff _radialfalloff 5e+05 0.0 1.0 0.0 _returnvalue _returnvalue_2 "Field_FallOff_None"))
  (Class|FieldSystemComponent|ApplyPhysicsField _fieldsystemcomponent true "Field_ExternalClusterStrain" 0 _returnvalue_3)
  (Class|FieldSystemComponent|ApplyPhysicsField _fieldsystemcomponent true "Field_LinearVelocity" 0 (Field|SetCullingField (Variables|Default|GetCullingField) _returnvalue_3 (Field|SetRadialVector (Variables|Default|GetRadialVector) 7.5e+02 _returnvalue_2) "Field_Culling_Outside"))
  (Actor|DestroyActor))

(event EventBeginPlay)

(event Collision|EventActorBeginOverlap
  (params (OtherActor :type Actor%20Object%20Reference)))

(event EventTick
  (params (DeltaSeconds :type Float%20%28single-precision%29)))

(fn ConstructionScript)