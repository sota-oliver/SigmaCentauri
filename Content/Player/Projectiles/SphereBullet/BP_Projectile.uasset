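; BP_Projectile is a sphere bullet projectile that detonates on impact.
; On a hit with anything other than itself, it spawns a Trigger_BP at the hit location, calls Explode on it and destroys itself.
; Its Sphere overlap also destroys it, without exploding, when the other actor's display name contains "SmallShip", a case-sensitive string match rather than a class check.
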(event OnComponentBeginOverlap(Sphere)
  (params (OverlappedComponent :type Primitive%20Component%20Object%20Reference) (OtherActor :type Actor%20Object%20Reference) (OtherComp :type Primitive%20Component%20Object%20Reference) (OtherBodyIndex :type Integer) (bFromSweep :type Boolean) (SweepResult :type Hit%20Result%20Structure%20%28by%20ref%29))
  (if (Utilities|String|Contains (Utilities|GetDisplayName OtherActor) "SmallShip" true)
    (Actor|DestroyActor)))

(event Collision|EventHit
  (params (MyComp :type Primitive%20Component%20Object%20Reference) (Other :type Actor%20Object%20Reference) (OtherComp :type Primitive%20Component%20Object%20Reference) (bSelfMoved :type Boolean) (HitLocation :type Vector :default "0, 0, 0") (HitNormal :type Vector :default "0, 0, 0") (NormalImpulse :type Vector :default "0, 0, 0") (Hit :type Hit%20Result%20Structure%20%28by%20ref%29))
  (if (not (== Other self))
    (bind _returnvalue (Game|SpawnActorfromClass "/Game/Player/Projectiles/SphereBullet/Trigger_BP.Trigger_BP_C" (Math|Transform|MakeTransform HitLocation "0, 0, 0" "1.000000,1.000000,1.000000") "Undefined" 0 0))
    (Default|Explode _returnvalue)
    (Actor|DestroyActor)))

(fn ConstructionScript)