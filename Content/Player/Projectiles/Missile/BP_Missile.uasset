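; Homing missile projectile that steers toward the closest actor tagged "Homing" and explodes on impact.
; From BeginPlay it repeatedly re-acquires a target by distance and feeds its scene component to ProjectileMovement as the homing target.
; A fast looping timer eases the missile's rotation toward that target.
; A hit spawns and detonates a Trigger_BP before destroying the missile, while sphere overlap with a "SmallShip"-named actor just destroys it.
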(event OnComponentBeginOverlap(Sphere)
  (params (OverlappedComponent :type Primitive%20Component%20Object%20Reference) (OtherActor :type Actor%20Object%20Reference) (OtherComp :type Primitive%20Component%20Object%20Reference) (OtherBodyIndex :type Integer) (bFromSweep :type Boolean) (SweepResult :type Hit%20Result%20Structure%20%28by%20ref%29))
  (if (Utilities|String|Contains (Utilities|GetDisplayName OtherActor) "SmallShip" true)
    (Actor|DestroyActor)))

(event Custom|LockOn
  (bind _projectilemovement (Variables|Default|GetProjectileMovement))
  (bind (_homingtarget _actor) (CallFunction|FindHomingTarget))
  (Variables|/Script/Engine.ProjectileMovementComponent|SetHomingTargetComponent _projectilemovement _homingtarget)
  (Variables|/Script/Engine.ProjectileMovementComponent|SetbIsHomingProjectile _projectilemovement true))

(event Custom|Rotate
  (Transformation|SetActorRotation (Math|Interpolation|RInterpTo (Transformation|GetActorRotation self) (Math|Rotator|FindLookatRotation (Transformation|GetActorLocation) (Transformation|GetActorLocation (stale Custom|LockOn _actor))) 0.2 0.1)))

(event EventBeginPlay
  (Utilities|Time|SetTimerbyEvent (delegate Custom|Rotate) 0.01 true)
  (CallFunction|Lockon :!label _label)
  (Utilities|FlowControl|Delay 0.2)
  (goto _label))

(event Collision|EventHit
  (params (MyComp :type Primitive%20Component%20Object%20Reference) (Other :type Actor%20Object%20Reference) (OtherComp :type Primitive%20Component%20Object%20Reference) (bSelfMoved :type Boolean) (HitLocation :type Vector :default "0, 0, 0") (HitNormal :type Vector :default "0, 0, 0") (NormalImpulse :type Vector :default "0, 0, 0") (Hit :type Hit%20Result%20Structure%20%28by%20ref%29))
  (if (not (== Other self))
    (bind _returnvalue (Game|SpawnActorfromClass "/Game/Player/Projectiles/SphereBullet/Trigger_BP.Trigger_BP_C" (Math|Transform|MakeTransform HitLocation "0, 0, 0" "1.000000,1.000000,1.000000") "Undefined" 0 0))
    (Default|Explode _returnvalue)
    (Actor|DestroyActor)))

(fn ConstructionScript)

(fn FindHomingTarget
  (bind _outactors (Actor|GetAllActorsOfClasswithTag "/Script/Engine.Actor" "Homing"))
  (for _array_element _outactors
    (if (< (Math|Vector|VectorLength (- (Transformation|GetActorLocation _array_element) (Transformation|GetActorLocation))) (Variables|Default|GetClosestDistance))
      (Variables|Default|SetClosestDistance (Math|Vector|VectorLength (- (Transformation|GetActorLocation _array_element) (Transformation|GetActorLocation))))
      (Variables|Default|SetHomingTarget _array_element)))
  (return (Actor|GetComponentbyClass (Variables|Default|GetHomingTarget) "/Script/Engine.SceneComponent") (Variables|Default|GetHomingTarget)))