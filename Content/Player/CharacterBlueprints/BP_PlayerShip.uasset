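; Player-controlled flying ship pawn with thrust, pitch, yaw and roll flight, plus guns, missiles and bombs.
; Tick moves it forward with drag-based slowdown and updates ammo and missile widgets.
; A timer offsets a dynamic crosshair by smoothed steering; alternating turrets and launchers aim through it, with timed reloads.
; Projectile hits drain shields before health, and shield impacts feed a material parameter collection; the death screen is never shown.
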(event OnComponentHit(CapsuleComponent)
  (params (HitComponent :type Primitive%20Component%20Object%20Reference) (OtherActor :type Actor%20Object%20Reference) (OtherComp :type Primitive%20Component%20Object%20Reference) (NormalImpulse :type Vector :default "0, 0, 0") (Hit :type Hit%20Result%20Structure%20%28by%20ref%29)))

(event OnComponentHit(StaticMesh1)
  (params (HitComponent :type Primitive%20Component%20Object%20Reference) (OtherActor :type Actor%20Object%20Reference) (OtherComp :type Primitive%20Component%20Object%20Reference) (NormalImpulse :type Vector :default "0, 0, 0") (Hit :type Hit%20Result%20Structure%20%28by%20ref%29))
  ;[1 0.006678 0 1 35] OnComponentHit (Health)
  (switch int (Variables|DynamicVariables|Shields|GetHitNumber)
    (:0
      (Rendering|Material|SetVectorParameterValue "/Game/Player/Shield/MPC_ShieldValues.MPC_ShieldValues" "Loc0" (Math|Conversions|ToLinearColor(Vector) (.location Hit)) :!class /Script/Engine.KismetMaterialLibrary)
      (Development|PrintString "CharacterShieldHit")
      (if (Utilities|String|Contains (Utilities|GetDisplayName (stale OnComponentHit(Mesh) OtherActor)) "Projectile" true)
        (if (== (Variables|Constants|GetShields) 0.0)
          (if (!= (Variables|Constants|GetHealth) 0.0)
            (Variables|Constants|SetHealth (- (Variables|Constants|GetHealth) 25.0))
            (if (== (Variables|Constants|GetHealth) 0.0)
              _))
          (else
            (Variables|Constants|SetShields (- (Variables|Constants|GetShields) 5e+01))))))))

(event OnComponentHit(Mesh)
  (params (HitComponent :type Primitive%20Component%20Object%20Reference) (OtherActor :type Actor%20Object%20Reference) (OtherComp :type Primitive%20Component%20Object%20Reference) (NormalImpulse :type Vector :default "0, 0, 0") (Hit :type Hit%20Result%20Structure%20%28by%20ref%29))
  ;[1 0.006678 0 1 35] OnComponentHit (Health)
  (if (Utilities|String|Contains (Utilities|GetDisplayName OtherActor) "Projectile" true)
    (if (== (Variables|Constants|GetShields) 0.0)
      (if (!= (Variables|Constants|GetHealth) 0.0)
        (Variables|Constants|SetHealth (- (Variables|Constants|GetHealth) 25.0))
        (if (== (Variables|Constants|GetHealth) 0.0)
          _))
      (else
        (Variables|Constants|SetShields (- (Variables|Constants|GetShields) 5e+01))))))

(event Custom|AlignDynamicCrosshair
  ;[1 1 1] Dynamic Crosshair
  (CallFunction|DynamicCrosshairMovement (stale Input|AxisEvents|InputAxisPitch _currentpitch) (stale Input|AxisEvents|InputAxisYaw _currentyaw)))

(event Custom|CustomEvent
  ;[0.9647 1 0 1 35] MissileReload (set to constant)
  (if (!= (Variables|DynamicVariables|Weapons|GetCurrentMissiles) 4)
    (if (not (Variables|WeaponTriggers|GetIsLaunching))
      (Variables|DynamicVariables|Weapons|SetCurrentMissiles (+ (Variables|DynamicVariables|Weapons|GetCurrentMissiles) 1)))))

(event Custom|ReloadAmmo
  ;[0.9647 1 0 1 35] AmmoReload (set to constant)
  (if (!= (Variables|DynamicVariables|Weapons|GetCurrentAmmo) 12)
    (if (not (Variables|WeaponTriggers|GetIsShooting))
      (Variables|DynamicVariables|Weapons|SetCurrentAmmo (+ (Variables|DynamicVariables|Weapons|GetCurrentAmmo) 1)))))

(event EventBeginPlay
  ;[1 1 1] EventBeginPlay
  (bind _output_get (Variables|DynamicVariables|Movement|SetThrustSpeed (Variables|Constants|GetMinThrustToNotFall)))
  (Variables|DynamicVariables|Movement|SetCurrentSpeed _output_get)
  ;[1 1 1] AmmoProjectileCountSetup
  (Variables|DynamicVariables|Weapons|SetCurrentAmmo (Math|Float|Truncate (Variables|Constants|GetMaxAmmo)))
  (Variables|Constants|SetMaxAmmoPercentage (/ 1e+02 (Variables|Constants|GetMaxAmmo)))
  ;[1 1 1] MissileProjectileCountSetup
  (Variables|DynamicVariables|Weapons|SetCurrentMissiles (Math|Float|Truncate (Variables|Constants|GetMaxMissiles)))
  ;[1 1 1] Create UI
  (CallFunction|CreateUI)
  ;[1 1 1] Dynamic Crosshair
  (Utilities|Time|SetTimerbyEvent (delegate Custom|AlignDynamicCrosshair) 0.01 true)
  ;[0.9647 1 0 1 35] AmmoReload (set to constant)
  (Utilities|Time|SetTimerbyEvent (delegate Custom|ReloadAmmo) 0.3 true)
  ;[0.9647 1 0 1 35] MissileReload (set to constant)
  (Utilities|Time|SetTimerbyEvent (delegate Custom|CustomEvent) 2.0 true))

(event EventTick
  (params (DeltaSeconds :type Float%20%28single-precision%29))
  (bind _currentammo (Variables|DynamicVariables|Weapons|GetCurrentAmmo))
  ;[1 1 1] EventTick
  (Private|UpdatePosition DeltaSeconds)
  (Private|PrintVariables)
  ;[1 1 1] Check Munitions
  (CallFunction|CheckMunitions _currentammo (Variables|DynamicVariables|Weapons|GetCurrentMissiles))
  ;[1 1 1] AmmoPercentage Calculation for Ammo widget
  (Variables|/Game/2D/YUGO_HUD/AmmoIndicator/W_AmmoProgressBar.W_AmmoProgressBar_C|SetPercentage (Variables|/Game/2D/YUGO_HUD/AmmoIndicator/W_AmmoMain.W_AmmoMain_C|GetW_AmmoProgressBar (Variables|Default|GetW_Ammo)) (/ (* (Math|Conversions|ToFloat(Integer) _currentammo) (Variables|Constants|GetMaxAmmoPercentage)) 1e+02))
  (CallFunction|ChangeMissileWidget))

(event Input|ActionEvents|InputActionDropBomb
  (params (Key :type Key%20Structure :default "None"))
  (bind _mesh (Variables|Character|GetMesh))
  ;[0 0.1626 1 1 35] Weapon systems
  (:Pressed
    (if (== (Variables|DynamicVariables|Weapons|GetCurrentBombs) 0)
      (Variables|Default|SetIsDroppingBombs false :!label _label)
      (else
        (Variables|Default|SetIsDroppingBombs true)
        (if (Variables|Default|GetIsDroppingBombs)
          (Game|SpawnActorfromClass "/Game/Player/Projectiles/Bomb/BP_Bomb.BP_Bomb_C" (Math|Transform|MakeTransform (Transformation|GetSocketLocation _mesh "Sphincter") (Transformation|GetSocketRotation _mesh "Sphincter") "1.000000,1.000000,1.000000") "Undefined" 0 0)))))
  (:Released
    (goto _label)))

(event Input|ActionEvents|InputActionLaunch
  (params (Key :type Key%20Structure :default "None"))
  ;[0 0.1626 1 1 35] Weapon systems
  ;;[1 1 1 1 35] Missile input
  (:Pressed
    (if (== (Variables|DynamicVariables|Weapons|GetCurrentMissiles) 0)
      (Variables|WeaponTriggers|SetIsLaunching false :!label _label)
      (else
        (Variables|WeaponTriggers|SetIsLaunching true)
        (if (Variables|WeaponTriggers|GetIsLaunching) :!label _label_2
          (if (Variables|WeaponTriggers|GetDualLauncherFiringSwitch)
            (CallFunction|SpawnandRotateMissile "MissileLauncherRight")
            (else
              (CallFunction|SpawnandRotateMissile "MissileLauncherLeft")))
          (Utilities|FlowControl|Delay 0.4)
          (goto _label_2)))))
  (:Released
    (goto _label)))

(event Input|ActionEvents|InputActionFrontCameraSwitch
  (params (Key :type Key%20Structure :default "None"))
  (bind _cameraboom (Variables|Camera|GetCameraBoom))
  (:Pressed
    (Variables|/Script/Engine.SpringArmComponent|SetCameraLagSpeed _cameraboom 0.0)
    (Variables|/Script/Engine.SpringArmComponent|SetCameraRotationLagSpeed _cameraboom 0.0)
    (Class|SceneComponent|AddLocalTransform _cameraboom (Math|Transform|MakeTransform "0, 0, 0" "0,180.000000, 0" "1.000000,1.000000,1.000000") false false)
    (Variables|/Script/Engine.SpringArmComponent|SetTargetArmLength _cameraboom 2e+02)))

(event Input|ActionEvents|InputActionShoot
  (params (Key :type Key%20Structure :default "None"))
  ;[0 0.1626 1 1 35] Weapon systems
  ;;[1 1 1 1 35] Shoot input
  (:Pressed
    (if (== (Variables|DynamicVariables|Weapons|GetCurrentAmmo) 0)
      (Variables|WeaponTriggers|SetIsShooting false :!label _label)
      (else
        (Variables|WeaponTriggers|SetIsShooting true)
        (if (Variables|WeaponTriggers|GetIsShooting) :!label _label_2
          (if (Variables|WeaponTriggers|GetDualTurretFiringSwitch)
            (CallFunction|SpawnandRotateProjectile "FrontLeftTurret_Socket")
            (else
              (CallFunction|SpawnandRotateProjectile "FrontRightTurret_Socket")))
          (Utilities|FlowControl|Delay 0.1)
          (goto _label_2)))))
  (:Released
    (goto _label)))

(event Input|AxisEvents|InputAxisThrust
  (params (AxisValue :type Float%20%28single-precision%29))
  ;[0 0.04167 0.001973 1 35] Movement
  ;;[1 1 1] Thrust input
  (Variables|DynamicVariables|Movement|SetThrustSpeed (Math|Float|Clamp(Float) (+ (* AxisValue (Utilities|Time|GetWorldDeltaSeconds) (Variables|Constants|GetThrustMultiplier)) (Variables|DynamicVariables|Movement|GetThrustSpeed)) 0.0 (Variables|Constants|GetMaxThrustSpeed))))

(event Input|AxisEvents|InputAxisYaw
  (params (AxisValue :type Float%20%28single-precision%29))
  ;[0 0.04167 0.001973 1 35] Movement
  ;;[1 1 1] Yaw input
  (bind _currentyaw (Private|UpdateYaw (Utilities|Time|GetWorldDeltaSeconds) AxisValue)))

(event Input|AxisEvents|InputAxisPitch
  (params (AxisValue :type Float%20%28single-precision%29))
  ;[0 0.04167 0.001973 1 35] Movement
  ;;[1 1 1] Pitch input
  (bind _currentpitch (Private|UpdatePitch (Utilities|Time|GetWorldDeltaSeconds) AxisValue)))

(event Input|AxisEvents|InputAxisRoll
  (params (AxisValue :type Float%20%28single-precision%29))
  ;[0 0.04167 0.001973 1 35] Movement
  ;;[1 1 1] Roll input
  (Private|UpdateRoll (Utilities|Time|GetWorldDeltaSeconds) AxisValue))

(fn ConstructionScript)

(fn UpdatePosition
  (params (DeltaSeconds :type Float%20%28double-precision%29))
  (Variables|DynamicVariables|Movement|SetCurrentSpeed (Math|Float|SelectFloat (Variables|DynamicVariables|Movement|GetThrustSpeed) (Math|Interpolation|FInterpTo (Variables|DynamicVariables|Movement|GetCurrentSpeed) (Variables|DynamicVariables|Movement|GetThrustSpeed) DeltaSeconds (Variables|Constants|GetDrag)) (< (Variables|DynamicVariables|Movement|GetThrustSpeed) (Variables|DynamicVariables|Movement|GetCurrentSpeed))))
  (LocalVariables|SetNewPosition (* (Transformation|GetActorForwardVector) (* (Variables|DynamicVariables|Movement|GetCurrentSpeed) DeltaSeconds)))
  (Variables|DynamicVariables|Movement|SetAppliedGravity (Math|Float|MapRangeClamped (Variables|DynamicVariables|Movement|GetCurrentSpeed) 0.0 (Variables|Constants|GetMinThrustToNotFall) (Variables|Constants|GetGravity) 0.0))
  (Transformation|AddActorWorldOffset (Math|Vector|MakeVector (.X (Math|Vector|BreakVector (LocalVariables|GetNewPosition))) (.Y (Math|Vector|BreakVector (LocalVariables|GetNewPosition))) (- (.Z (Math|Vector|BreakVector (LocalVariables|GetNewPosition))) DeltaSeconds))))

(fn UpdateYaw
  (params (DeltaSeconds :type Float%20%28double-precision%29) (Yaw :type Float%20%28double-precision%29))
  (Variables|DynamicVariables|Rotation|SetTargetYaw Yaw)
  (bind _output_get (Variables|DynamicVariables|Rotation|SetCurrentYaw (Math|Interpolation|FInterpTo (Variables|DynamicVariables|Rotation|GetCurrentYaw) (Variables|DynamicVariables|Rotation|GetTargetYaw) DeltaSeconds 1.0)))
  (Transformation|AddActorLocalRotation (Math|Rotator|MakeRotator 0.0 0.0 (* _output_get DeltaSeconds 1e+01)) false false)
  (return _output_get))

(fn UpdatePitch
  (params (DeltaSeconds :type Float%20%28double-precision%29) (Pitch :type Float%20%28double-precision%29))
  (Variables|DynamicVariables|Rotation|SetTargetPitch Pitch)
  (bind _output_get (Variables|DynamicVariables|Rotation|SetCurrentPitch (Math|Interpolation|FInterpTo (Variables|DynamicVariables|Rotation|GetCurrentPitch) (Variables|DynamicVariables|Rotation|GetTargetPitch) DeltaSeconds 1.0)))
  (Transformation|AddActorLocalRotation (Math|Rotator|MakeRotator 0.0 (* _output_get DeltaSeconds 1e+01) 0.0) false false)
  (return _output_get))

(fn UpdateRoll
  (params (DeltaSeconds :type Float%20%28double-precision%29) (Roll :type Float%20%28double-precision%29))
  (Variables|DynamicVariables|Rotation|SetTargetRoll Roll)
  (bind _output_get (Variables|DynamicVariables|Rotation|SetCurrentRoll (Math|Interpolation|FInterpTo (Variables|DynamicVariables|Rotation|GetCurrentRoll) (Variables|DynamicVariables|Rotation|GetTargetRoll) DeltaSeconds 1e+01)))
  (Transformation|AddActorLocalRotation (Math|Rotator|MakeRotator (* _output_get DeltaSeconds 5e+01) 0.0 0.0) false false)
  (return _output_get))

(fn PrintVariables
  (Utilities|FlowControl|Sequence
    (:then_0
      (Development|PrintString (Utilities|String|Append "ThrustSpeed: " (Utilities|String|ToString(Float) (Variables|DynamicVariables|Movement|GetThrustSpeed))) true true "(R=0.000000,G=0.660000,B=1.000000,A=1.000000)" 0.0))
    (:then_1
      (Development|PrintString (Utilities|String|Append "CurrentSpeed: " (Utilities|String|ToString(Float) (Variables|DynamicVariables|Movement|GetCurrentSpeed))) true true "(R=0.000000,G=0.660000,B=1.000000,A=1.000000)" 0.0))
    (:then_4
      (Development|PrintString (Utilities|String|Append "Health: " (Utilities|String|ToString(Float) (Variables|Constants|GetHealth))) true true "(R=0.002387,G=0.166667,B=0.000000,A=1.000000)" 0.0))
    (:then_5
      (Development|PrintString (Utilities|String|Append "Shields: " (Utilities|String|ToString(Float) (Variables|Constants|GetShields))) true true "(R=0.002387,G=0.166667,B=0.000000,A=1.000000)" 0.0))
    (:then_6
      (Development|PrintString (Utilities|String|Append "Ammo: " (Utilities|String|ToString(Integer) (Variables|DynamicVariables|Weapons|GetCurrentAmmo))) true true "(R=0.000000,G=0.660000,B=1.000000,A=1.000000)" 0.0))
    (:then_7
      (Development|PrintString (Utilities|String|Append "Missiles: " (Utilities|String|ToString(Integer) (Variables|DynamicVariables|Weapons|GetCurrentMissiles))) true true "(R=0.000000,G=0.660000,B=1.000000,A=1.000000)" 0.0))))

(fn CreateUI
  (bind _returnvalue (UserInterface|CreateWidget "/Game/2D/YUGO_HUD/DynamicMouseCrosshair/W_DynamicMouseCrosshair.W_DynamicMouseCrosshair_C"))
  (UserInterface|Viewport|AddtoViewport _returnvalue 0)
  (Variables|Default|SetW_DynamicMouseCrosshair _returnvalue)
  (bind _returnvalue_2 (UserInterface|CreateWidget "/Game/2D/YUGO_HUD/AmmoIndicator/W_AmmoMain.W_AmmoMain_C"))
  (bind _output_get (Variables|Default|SetW_Ammo _returnvalue_2))
  (UserInterface|Viewport|AddtoViewport _output_get 0)
  (bind _returnvalue_3 (UserInterface|CreateWidget "/Game/2D/YUGO_HUD/W_MissileMain.W_MissileMain_C"))
  (bind _output_get_2 (Variables|Default|SetW_Missile _returnvalue_3))
  (UserInterface|Viewport|AddtoViewport _output_get_2 0)
  (bind _returnvalue_4 (UserInterface|CreateWidget "/Game/2D/POPUP.POPUP_C"))
  (Variables|Default|SetW_DeathScreen _returnvalue_4))

(fn DynamicCrosshairMovement
  (params (A :type Float%20%28double-precision%29) (A2 :type Float%20%28double-precision%29))
  (bind _returnvalue (Viewport|GetViewportSize))
  (bind _returnvalue_2 (* A2 1e+02))
  (bind _returnvalue_3 (* A -1e+02))
  (bind _returnvalue_4 (/ (.y _returnvalue) 2.0))
  (bind _returnvalue_5 (/ (.x _returnvalue) 2.0))
  (bind _returnvalue_6 (+ _returnvalue_4 _returnvalue_3))
  (bind _returnvalue_7 (+ _returnvalue_5 _returnvalue_2))
  (Variables|DynamicVariables|Rotation|SetDynamicCrosshairPositionX _returnvalue_7)
  (Variables|DynamicVariables|Rotation|SetDynamicCrosshairPositionY _returnvalue_6)
  (Class|UserWidget|SetPositioninViewport (Variables|Default|GetW_DynamicMouseCrosshair) (Math|Vector2D|MakeVector2D _returnvalue_7 _returnvalue_6) true))

(fn SpawnandRotateProjectile
  (params (InSocketName :type Name))
  (bind _returnvalue (Game|GetPlayerController 0))
  (bind _dynamiccrosshairpositionx (Variables|DynamicVariables|Rotation|GetDynamicCrosshairPositionX))
  (bind _dynamiccrosshairpositiony (Variables|DynamicVariables|Rotation|GetDynamicCrosshairPositionY))
  (bind _mesh (Variables|Character|GetMesh))
  (bind _mesh_2 (Variables|Character|GetMesh))
  (bind _returnvalue_2 (Transformation|GetSocketTransform _mesh InSocketName "RTS_World"))
  (bind _returnvalue_3 (Transformation|GetSocketTransform _mesh_2 InSocketName "RTS_World"))
  (bind _returnvalue_4 (+ _dynamiccrosshairpositiony 2e+01))
  (bind _returnvalue_5 (+ _dynamiccrosshairpositionx 2e+01))
  (bind (_worldposition _worlddirection) (Class|GameplayStatics|DeprojectScreentoWorld _returnvalue (Math|Vector2D|MakeVector2D _returnvalue_5 _returnvalue_4)))
  (bind _returnvalue_6 (* _worlddirection 6.5e+04))
  (bind _returnvalue_7 (+ _worldposition _returnvalue_6))
  (bind _outhit (Collision|LineTraceByChannel _worldposition _returnvalue_7 "TraceTypeQuery1" false 0 "None" true "(R=1.000000,G=0.000000,B=0.000000,A=1.000000)" "(R=0.000000,G=1.000000,B=0.000000,A=1.000000)" 0.2))
  (if (.bBlockingHit (Collision|BreakHitResult _outhit))
    (Game|SpawnActorfromClass "/Game/Player/Projectiles/SphereBullet/BP_Projectile.BP_Projectile_C" (Math|Transform|MakeTransform (.location _returnvalue_3) (Math|Rotator|FindLookatRotation (.location _returnvalue_3) (.Location (Collision|BreakHitResult _outhit))) (.scale _returnvalue_3)) "Undefined" (Variables|Default|GetPlayerShipActor) 0)
    (Variables|DynamicVariables|Weapons|SetCurrentAmmo (- (Variables|DynamicVariables|Weapons|GetCurrentAmmo) 1))
    (if (Variables|WeaponTriggers|GetDualTurretFiringSwitch)
      (Variables|WeaponTriggers|SetDualTurretFiringSwitch false)
      (else
        (Variables|WeaponTriggers|SetDualTurretFiringSwitch true)))
    ;[1 1 1] Emmit sound when shooting (maybe neccessary to duplicate in case of shooting delay)
    (Audio|SpawnSoundatLocation "/Game/Metasound/Yugo22_Sounds/MS_Yugo22BulletFire.MS_Yugo22BulletFire" (Transformation|GetSocketLocation (Variables|Character|GetMesh) "None") "0, 0, 0" 1.0 1.0 0.0 0 0)
    (else
      (Game|SpawnActorfromClass "/Game/Player/Projectiles/SphereBullet/BP_Projectile.BP_Projectile_C" (Math|Transform|MakeTransform (.location _returnvalue_2) (Math|Rotator|FindLookatRotation (.location _returnvalue_2) _returnvalue_7) (.scale _returnvalue_2)) "Undefined" (Variables|Default|GetPlayerShipActor) 0)
      (Variables|DynamicVariables|Weapons|SetCurrentAmmo (- (Variables|DynamicVariables|Weapons|GetCurrentAmmo) 1))
      (if (Variables|WeaponTriggers|GetDualTurretFiringSwitch)
        (Variables|WeaponTriggers|SetDualTurretFiringSwitch false)
        (else
          (Variables|WeaponTriggers|SetDualTurretFiringSwitch true)))
      ;[1 1 1] Emmit sound when shooting (maybe neccessary to duplicate in case of shooting delay)
      (Audio|SpawnSoundatLocation "/Game/Metasound/Yugo22_Sounds/MS_Yugo22BulletFire.MS_Yugo22BulletFire" (Transformation|GetSocketLocation (Variables|Character|GetMesh) "None") "0, 0, 0" 1.0 1.0 0.0 0 0))))

(fn SpawnandRotateMissile
  (params (InSocketName :type Name))
  (bind _returnvalue (Game|GetPlayerController 0))
  (bind _dynamiccrosshairpositionx (Variables|DynamicVariables|Rotation|GetDynamicCrosshairPositionX))
  (bind _dynamiccrosshairpositiony (Variables|DynamicVariables|Rotation|GetDynamicCrosshairPositionY))
  (bind _mesh (Variables|Character|GetMesh))
  (bind _returnvalue_2 (Transformation|GetSocketTransform _mesh InSocketName "RTS_World"))
  (bind _returnvalue_3 (+ _dynamiccrosshairpositiony 2e+01))
  (bind _returnvalue_4 (+ _dynamiccrosshairpositionx 2e+01))
  (bind (_worldposition _worlddirection) (Class|GameplayStatics|DeprojectScreentoWorld _returnvalue (Math|Vector2D|MakeVector2D _returnvalue_4 _returnvalue_3)))
  (Game|SpawnActorfromClass "/Game/Player/Projectiles/Missile/BP_Missile.BP_Missile_C" (Math|Transform|MakeTransform (.location _returnvalue_2) (Math|Rotator|FindLookatRotation (.location _returnvalue_2) (+ _worldposition (* _worlddirection 6.5e+04))) (.scale _returnvalue_2)) "Undefined" (Variables|Default|GetPlayerShipActor) 0)
  (Variables|DynamicVariables|Weapons|SetCurrentMissiles (- (Variables|DynamicVariables|Weapons|GetCurrentMissiles) 1))
  (if (Variables|WeaponTriggers|GetDualLauncherFiringSwitch)
    (Variables|WeaponTriggers|SetDualLauncherFiringSwitch false)
    (else
      (Variables|WeaponTriggers|SetDualLauncherFiringSwitch true))))

(fn CheckMunitions
  (params (Ammo :type Integer) (Missiles :type Integer))
  (Utilities|FlowControl|Sequence
    (:then_0
      (if (== Ammo 0)
        (Variables|WeaponTriggers|SetIsShooting false)))
    (:then_1
      (if (== Missiles 0)
        (Variables|WeaponTriggers|SetIsLaunching false)))))

(fn ChangeMissileWidget
  (bind _w_missile (Variables|Default|GetW_Missile))
  (bind _w_missile_2 (Variables|Default|GetW_Missile))
  (bind _w_missile_3 (Variables|Default|GetW_Missile))
  (bind _w_missile_4 (Variables|Default|GetW_Missile))
  (if (== (Variables|DynamicVariables|Weapons|GetCurrentMissiles) 4)
    (Variables|/Game/2D/YUGO_HUD/W_MissileMain.W_MissileMain_C|SetCheck00 _w_missile_2 true)
    (Variables|/Game/2D/YUGO_HUD/W_MissileMain.W_MissileMain_C|SetCheck01 _w_missile_2 true)
    (Variables|/Game/2D/YUGO_HUD/W_MissileMain.W_MissileMain_C|SetCheck02 _w_missile_2 true)
    (Variables|/Game/2D/YUGO_HUD/W_MissileMain.W_MissileMain_C|SetCheck03 _w_missile_2 true)
    (elif (>= (Variables|DynamicVariables|Weapons|GetCurrentMissiles) 3)
      (Variables|/Game/2D/YUGO_HUD/W_MissileMain.W_MissileMain_C|SetCheck00 _w_missile_3 false)
      (Variables|/Game/2D/YUGO_HUD/W_MissileMain.W_MissileMain_C|SetCheck01 _w_missile_3 true)
      (Variables|/Game/2D/YUGO_HUD/W_MissileMain.W_MissileMain_C|SetCheck02 _w_missile_3 true)
      (Variables|/Game/2D/YUGO_HUD/W_MissileMain.W_MissileMain_C|SetCheck03 _w_missile_3 true)
      (elif (>= (Variables|DynamicVariables|Weapons|GetCurrentMissiles) 2)
        (Variables|/Game/2D/YUGO_HUD/W_MissileMain.W_MissileMain_C|SetCheck00 _w_missile_4 false)
        (Variables|/Game/2D/YUGO_HUD/W_MissileMain.W_MissileMain_C|SetCheck01 _w_missile_4 false)
        (Variables|/Game/2D/YUGO_HUD/W_MissileMain.W_MissileMain_C|SetCheck02 _w_missile_4 true)
        (Variables|/Game/2D/YUGO_HUD/W_MissileMain.W_MissileMain_C|SetCheck03 _w_missile_4 true)
        (elif (>= (Variables|DynamicVariables|Weapons|GetCurrentMissiles) 1)
          (Variables|/Game/2D/YUGO_HUD/W_MissileMain.W_MissileMain_C|SetCheck00 _w_missile false)
          (Variables|/Game/2D/YUGO_HUD/W_MissileMain.W_MissileMain_C|SetCheck01 _w_missile false)
          (Variables|/Game/2D/YUGO_HUD/W_MissileMain.W_MissileMain_C|SetCheck02 _w_missile false)
          (Variables|/Game/2D/YUGO_HUD/W_MissileMain.W_MissileMain_C|SetCheck03 _w_missile true)
          (else
            (Variables|/Game/2D/YUGO_HUD/W_MissileMain.W_MissileMain_C|SetCheck00 _w_missile false)
            (Variables|/Game/2D/YUGO_HUD/W_MissileMain.W_MissileMain_C|SetCheck01 _w_missile false)
            (Variables|/Game/2D/YUGO_HUD/W_MissileMain.W_MissileMain_C|SetCheck02 _w_missile false)
            (Variables|/Game/2D/YUGO_HUD/W_MissileMain.W_MissileMain_C|SetCheck03 _w_missile false)))))))